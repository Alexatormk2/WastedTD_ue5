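; Base enemy for a tower defense game that walks toward the player's base and trades health for money or damage.
; On possession it caches its AI controller and, a tick later, orders it to move to the base location held by the game mode.
; Lethal damage pays its money reward to the game mode and destroys it.
; DealDamage damages the game mode and destroys the enemy without a reward.
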(event `self.ReceiveBeginPlay`
  (bind _asgm_tower_defense (cast `/Game/blueprints/GM_towerDefense` (`GameplayStatics.GetGameMode`)))
  (set `self.GM_towerDefense` _asgm_tower_defense))

(event `self.ReceivePossessed`
  (params (NewController :type "Controller Object Reference"))
  (bind _asaic_enemy (cast `/Game/blueprints/enemys/AIC_enemy` NewController))
  (set `self.Aicenemy` _asaic_enemy)
  (`KismetSystemLibrary.DelayUntilNextTick`)
  (`self.MoveToGoal` (`/Game/blueprints/GM_towerDefense.baseloc` (`self.GM_towerDefense`))))

(fn `DealDamage`
  (`/Game/blueprints/GM_towerDefense.ReceiveDamage` (`self.GM_towerDefense`) (`self.Damage`))
  (`self.K2_DestroyActor`))

(fn `MoveToGoal`
  (params (GetLocation :type "Vector Structure"))
  (`/Game/blueprints/enemys/AIC_enemy.MoveToGoalAi` (`self.Aicenemy`) GetLocation))

(fn `ReceiveDamage`
  (params (Damage :type Integer))
  (bind _output_get (set `self.HealthPoints` (- (`self.HealthPoints`) Damage)))
  (if (<= _output_get 0)
    (`/Game/blueprints/GM_towerDefense.Add money` (`self.GM_towerDefense`) (`self.Money`))
    (`self.K2_DestroyActor`)))

(fn `UserConstructionScript`)