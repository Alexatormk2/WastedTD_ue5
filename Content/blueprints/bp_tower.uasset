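; Tower actor that automatically fires homing projectiles at bp_baseenemy actors within its detection sphere.
; Sphere overlaps maintain an Enemies array, and the first entry starts a looping Shoot timer at RateOfFire.
; Each shot spawns a projectile at the shooting point, homing on the capsule of the enemy at Index and carrying the tower's Damage.
; The timer pauses when a shot finds no enemies and resumes on a later entry.
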(event `self.Sphere.OnComponentBeginOverlap`
  (params (OverlappedComponent :type "PrimitiveComponent Object Reference") (OtherActor :type "Actor Object Reference") (OtherComp :type "PrimitiveComponent Object Reference") (OtherBodyIndex :type Integer) (bFromSweep :type Boolean) (SweepResult :type "HitResult Structure (by ref)"))
  (bind _asbp_baseenemy (cast `/Game/blueprints/enemys/bp_baseenemy` OtherActor))
  (`KismetArrayLibrary.Array_Add` (`self.Enemies`) _asbp_baseenemy)
  (if (`self.shooting`)
    (if (`KismetSystemLibrary.K2_IsValidTimerHandle` (`self.shoot timer hande`))
      (`KismetSystemLibrary.K2_UnPauseTimerHandle` (`self.shoot timer hande`)))
    (else
      (set `self.shooting` true)
      (bind _returnvalue (`KismetSystemLibrary.K2_SetTimerDelegate` (delegate `Shoot`) (`self.rate of fire`) true))
      (set `self.shoot timer hande` _returnvalue))))

(event `Shoot`
  (if (> (`KismetArrayLibrary.Array_Length` (`self.Enemies`)) 0)
    (bind _returnvalue (`|SpawnActorFromClass` (`self.proyectile`) (`KismetMathLibrary.MakeTransform` (`SceneComponent.K2_GetComponentLocation` (`self.shootingpoint`))) "AdjustIfPossibleButAlwaysSpawn" "MultiplyWithRoot" null null))
    (set `ProjectileMovementComponent.HomingTargetComponent` (`Character.CapsuleComponent` (`|GetArrayItem` (`self.Enemies`) (`self.Index`))) (`/Game/blueprints/bp_poyectile.ProjectileMovement` _returnvalue))
    (set `/Game/blueprints/bp_poyectile.damage` (`self.damage`) _returnvalue)
    (else
      (`KismetSystemLibrary.K2_PauseTimerHandle` (`self.shoot timer hande`)))))

(event `self.Sphere.OnComponentEndOverlap`
  (params (OverlappedComponent :type "PrimitiveComponent Object Reference") (OtherActor :type "Actor Object Reference") (OtherComp :type "PrimitiveComponent Object Reference") (OtherBodyIndex :type Integer))
  (bind _asbp_baseenemy (cast `/Game/blueprints/enemys/bp_baseenemy` OtherActor))
  (`KismetArrayLibrary.Array_RemoveItem` (`self.Enemies`) _asbp_baseenemy))

(fn `UserConstructionScript`)