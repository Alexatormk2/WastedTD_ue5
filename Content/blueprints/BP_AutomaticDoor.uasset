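; Automatic door Blueprint that moves its Plane vertically as a BP_TopDownCharacter enters or leaves the Box overlap.
; Each overlap starts its own looping timer that steps a shared Percentage and lerps the Plane's relative Z, clearing itself at full progress.
; Both lerps start from zero, so closing jumps down from the raised position, and neither timer cancels the other.
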(event `CustomEvent`
  ; open door
  (if (>= (`self.percentage`) 1.0)
    (`KismetSystemLibrary.K2_ClearAndInvalidateTimerHandle` (stale `self.Box.OnComponentBeginOverlap` _returnvalue))
    (set `self.percentage` 0.0)
    (else
      (set `self.percentage` (+ 0.01 (`self.percentage`)))
      (`SceneComponent.K2_SetRelativeLocation` (`self.Plane`) (`KismetMathLibrary.MakeVector` 0.0 0.0 (`KismetMathLibrary.Lerp` 0.0 260.0 (`self.percentage`))) false false))))

(event `self.Box.OnComponentBeginOverlap`
  (params (OverlappedComponent :type "PrimitiveComponent Object Reference") (OtherActor :type "Actor Object Reference") (OtherComp :type "PrimitiveComponent Object Reference") (OtherBodyIndex :type Integer) (bFromSweep :type Boolean) (SweepResult :type "HitResult Structure (by ref)"))
  ; open door
  (cast `/Game/TopDown/Blueprints/BP_TopDownCharacter` OtherActor)
  (bind _returnvalue (`KismetSystemLibrary.K2_SetTimerDelegate` (delegate `CustomEvent`) 0.01 true)))

(event `CustomEvent_1`
  ; closse door
  (if (>= (`self.percentage`) 1.0)
    (`KismetSystemLibrary.K2_ClearAndInvalidateTimerHandle` (stale `self.Box.OnComponentEndOverlap` _returnvalue))
    (set `self.percentage` 0.0)
    (else
      (set `self.percentage` (+ (`self.percentage`) 0.01))
      (`SceneComponent.K2_SetRelativeLocation` (`self.Plane`) (`KismetMathLibrary.MakeVector` 0.0 0.0 (`KismetMathLibrary.Lerp` 0.0 -20.0 (`self.percentage`))) false false))))

(event `self.Box.OnComponentEndOverlap`
  (params (OverlappedComponent :type "PrimitiveComponent Object Reference") (OtherActor :type "Actor Object Reference") (OtherComp :type "PrimitiveComponent Object Reference") (OtherBodyIndex :type Integer))
  ; closse door
  (cast `/Game/TopDown/Blueprints/BP_TopDownCharacter` OtherActor)
  (bind _returnvalue (`KismetSystemLibrary.K2_SetTimerDelegate` (delegate `CustomEvent_1`) 0.01 true)))

(fn `UserConstructionScript`)