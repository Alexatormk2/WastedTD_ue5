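; BP_TowerGatling is a tower that fires homing projectiles at enemies inside its detection sphere.
; Sphere overlaps add and remove BP_Baseenemy actors in the Enemies array, and entries start or resume a looping RateOfFire timer.
; Each tick of that timer spawns a projectile at Shootingpoint, passing it Damage and the indexed enemy's capsule as homing target.
; The timer pauses when it fires with no enemies in range.
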(event `self.Sphere.OnComponentBeginOverlap`
  (params (OverlappedComponent :type "PrimitiveComponent Object Reference") (OtherActor :type "Actor Object Reference") (OtherComp :type "PrimitiveComponent Object Reference") (OtherBodyIndex :type Integer) (bFromSweep :type Boolean) (SweepResult :type "HitResult Structure (by ref)"))
  (bind _asbp_baseenemy (cast `/Game/blueprints/enemys/BP_Baseenemy` OtherActor))
  (`KismetArrayLibrary.Array_Add` (`self.Enemies`) _asbp_baseenemy)
  (if (`self.Shooting`)
    (if (`KismetSystemLibrary.K2_IsValidTimerHandle` (`self.Shoot timer hande`))
      (`KismetSystemLibrary.K2_UnPauseTimerHandle` (`self.Shoot timer hande`)))
    (else
      (set `self.Shooting` true)
      (bind _returnvalue (`KismetSystemLibrary.K2_SetTimerDelegate` (delegate `Shoot`) (`self.Rate of fire`) true))
      (set `self.Shoot timer hande` _returnvalue))))

(event `Shoot`
  (if (> (`KismetArrayLibrary.Array_Length` (`self.Enemies`)) 0)
    (`GameplayStatics.PlaySoundAtLocation` "/Game/blueprints/audio/vrocweaa.vrocweaa" (0.0 0.0 0.0) (struct) 1.0 1.0 0.0 null null null null)
    (bind _returnvalue (`|SpawnActorFromClass` (`self.Proyectile`) (`KismetMathLibrary.MakeTransform` (`SceneComponent.K2_GetComponentLocation` (`self.shootingpoint`))) "AdjustIfPossibleButAlwaysSpawn" "MultiplyWithRoot" null null))
    (set `ProjectileMovementComponent.HomingTargetComponent` (`Character.CapsuleComponent` (`|GetArrayItem` (`self.Enemies`) (`self.Index`))) (`/Game/blueprints/BP_Proyectile.ProjectileMovement` _returnvalue))
    (set `/Game/blueprints/BP_Proyectile.Damage` (`self.Damage`) _returnvalue)
    (else
      (`KismetSystemLibrary.K2_PauseTimerHandle` (`self.Shoot timer hande`)))))

(event `self.Sphere.OnComponentEndOverlap`
  (params (OverlappedComponent :type "PrimitiveComponent Object Reference") (OtherActor :type "Actor Object Reference") (OtherComp :type "PrimitiveComponent Object Reference") (OtherBodyIndex :type Integer))
  (bind _asbp_baseenemy (cast `/Game/blueprints/enemys/BP_Baseenemy` OtherActor))
  (`KismetArrayLibrary.Array_RemoveItem` (`self.Enemies`) _asbp_baseenemy))

(fn `UserConstructionScript`)