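; Tower defense game mode that tracks money, health, waves and living enemies, and decides victory or defeat.
; It creates the game interface widget on BeginPlay and pushes money, health and wave changes to it.
; Damage that drops health to zero pauses the game and shows Game Over.
; Enemies register in a unique list; removing the last once the all-spawned flag is set pauses and shows Victory.
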(event `self.ReceiveBeginPlay`
  (bind _returnvalue (`|CreateWidget` "/Game/blueprints/widgets/WBP_GameInterface.WBP_GameInterface_C"))
  (bind _output_get (set `self.WBP_GameInterface` _returnvalue))
  (`UserWidget.AddToViewport` _output_get 0))

(fn `Add money`
  (params (Money :type Integer))
  (bind _output_get (set `self.Money` (+ (`self.Money`) Money)))
  (`/Game/blueprints/widgets/WBP_GameInterface.Update Money Text` (`self.WBP_GameInterface`) _output_get))

(fn `AdToListEnemy`
  (params (enemy :type "/Game/blueprints/enemys/bp_baseenemy Object Reference (by ref)"))
  (`KismetArrayLibrary.Array_AddUnique` (`self.Enemy`) enemy))

(fn `EnemyDeadWarning`
  (params (enemy :type "/Game/blueprints/enemys/bp_baseenemy Object Reference"))
  (bind _enemy (`self.Enemy`))
  (bind _allenemyspaw (`self.ALLenemySpaw`))
  (`KismetArrayLibrary.Array_RemoveItem` _enemy enemy)
  (`KismetSystemLibrary.PrintString` (`KismetStringLibrary.Conv_BoolToString` _allenemyspaw) true true (struct :`R` 0.036342 :`G` 1.0 :`A` 1.0) 5.0)
  (if (and _allenemyspaw (`KismetArrayLibrary.Array_IsEmpty` _enemy))
    (`self.Victory`)))

(fn `LooseGame`
  (`GameplayStatics.SetGamePaused` true)
  (bind _returnvalue (`|CreateWidget` "/Game/blueprints/widgets/WBP_GameOver.WBP_GameOver_C"))
  (`UserWidget.AddToViewport` _returnvalue 0))

(fn `ReceiveDamage`
  (params (Damage :type Integer))
  (bind _output_get (set `self.HealthPoints` (- (`self.HealthPoints`) Damage)))
  (`/Game/blueprints/widgets/WBP_GameInterface.Update Health Text` (`self.WBP_GameInterface`) _output_get)
  (if (<= _output_get 0)
    (`self.LooseGame`)))

(fn `UpdateWave`
  (bind _result (`/Engine/EditorBlueprintResources/StandardMacros.IncrementInt` (`self.wave`))
    (:`  `
      (`/Game/blueprints/widgets/WBP_GameInterface.UpdateWave` (`self.WBP_GameInterface`) _result))))

(fn `UserConstructionScript`)

(fn `Victory`
  (`GameplayStatics.SetGamePaused` true)
  (bind _returnvalue (`|CreateWidget` "/Game/blueprints/widgets/WBP_Victory.WBP_Victory_C"))
  (`UserWidget.AddToViewport` _returnvalue 0))