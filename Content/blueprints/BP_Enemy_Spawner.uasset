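; Enemy spawner actor that runs through a list of enemy waves, starting at BeginPlay and spawning each wave at its own location and rotation.
; StarterArray starts a looping timer from the current wave's start delay and spawn interval.
; Each Spawner tick spawns that wave's enemy class until its count is reached, then clears the timer, resets the counter and advances to the next wave until none remain.
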(event `StarterArray`
  (bind _enemywave (`self.EnemyWave`))
  (bind (_output_num_enemy _output_enemy_type _output_waveenemyspawtimer _output_nextwavetimer) (break `/Game/blueprints/S_Enemy_Wave` (`|GetArrayItem` _enemywave (`self.Index_0`))))
  (if (> (`KismetArrayLibrary.Array_Length` _enemywave) (`self.Index_0`))
    (bind _returnvalue (`KismetSystemLibrary.K2_SetTimerDelegate` (delegate `Spawner`) _output_waveenemyspawtimer true false _output_nextwavetimer))
    (elif (`KismetSystemLibrary.K2_IsValidTimerHandle` (`self.Handle`))
      (`KismetSystemLibrary.K2_ClearAndInvalidateTimerHandle` _returnvalue))))

(event `Spawner`
  (bind (_output_num_enemy _output_enemy_type _output_waveenemyspawtimer _output_nextwavetimer) (break `/Game/blueprints/S_Enemy_Wave` (`|GetArrayItem` (`self.EnemyWave`) (`self.Index_0`))))
  (if (< (`self.Contador`) _output_num_enemy)
    (bind _result (`/Engine/EditorBlueprintResources/StandardMacros.IncrementInt` (`self.Contador`))
      (:`  `
        (set `self.Contador` _result)
        (`|SpawnActorFromClass` _output_enemy_type (`KismetMathLibrary.MakeTransform` (`self.K2_GetActorLocation`) (`self.K2_GetActorRotation`)) "AdjustIfPossibleButAlwaysSpawn" "MultiplyWithRoot" null null)))
    (else
      (`KismetSystemLibrary.K2_ClearAndInvalidateTimerHandle` (`self.Handle`))
      (`/Engine/EditorBlueprintResources/StandardMacros.IncrementInt` (`self.Index_0`)
        (:`  `
          (set `self.Contador` 0)
          (`self.StarterArray`))))))

(event `self.ReceiveBeginPlay`
  (`self.StarterArray`))

(fn `UserConstructionScript`)